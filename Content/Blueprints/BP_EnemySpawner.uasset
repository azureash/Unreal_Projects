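; Destructible enemy spawner actor that keeps producing batches of enemies until damage drains its health and destroys it.
; BeginPlay spawns the first batch at SpawnPoint2 and caches BP_GameModeBase.
; SpawnEnemy then re-triggers itself after a delay at a random one of two spawn points while EnemiesAlive is below MaxEnemies.
; At the cap, ShouldSpawn polls on the same delay until there is room to spawn again.
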(event `/Game/Blueprints/BP_PlayerDamage_Interface.HitPlayer`
  (params (Damage :type Integer))
  ;[1 1 1] Enemy Health System
  (bind _output_get (set `self.Health` (- (`self.Health`) Damage)))
  (if (<= _output_get 0)
    (`self.K2_DestroyActor`)))

(event `self.ReceiveBeginPlay`
  ;[1 1 1] Spawn enemy Logic
  ;;[1 1 1] Spawn First Enemy
  (`|ExecutionSequence`
    (:`then_0`
      (`self.Event SpawnEnemy` (`self.Enemy`) (`KismetMathLibrary.MakeTransform` (`SceneComponent.K2_GetComponentLocation` (`self.SpawnPoint2`)) (struct :`Yaw` -90.0)) (`self.Number Of Enemies`)))
    (:`then_1`
      (bind _asbp_game_mode_base (cast `/Game/Blueprints/BP_GameModeBase` (`GameplayStatics.GetGameMode`)))
      (set `self.As BP Game Mode Base` _asbp_game_mode_base))))

(event `Event SpawnEnemy`
  (params (Enemy :type "Actor Class Reference") (SpawnTransform :type "Transform Structure") (`Number Of Enemies` :type Integer))
  (bind _as_bp_game_mode_base (`self.As BP Game Mode Base`))
  ;[1 1 1] Spawn enemy Logic
  ;;[1 1 1] Spawn Enemies Over Time
  (for _ (range `Number Of Enemies`)
    (`|SpawnActorFromClass` Enemy SpawnTransform "AdjustIfPossibleButAlwaysSpawn" "OverrideRootScale" null null))
  (`KismetSystemLibrary.Delay` (`self.Spawn Delay`))
  (if (< (`/Game/Blueprints/BP_GameModeBase.Enemies Alive` _as_bp_game_mode_base) (`/Game/Blueprints/BP_GameModeBase.Max Enemies` _as_bp_game_mode_base))
    (`self.Event SpawnEnemy` (`self.Enemy`) (`KismetMathLibrary.MakeTransform` (`SceneComponent.K2_GetComponentLocation` (`KismetArrayLibrary.Array_Random` (`|MakeArray` (`self.SpawnPoint2`) (`self.SpawnPoint1`)))) (struct :`Yaw` -90.0)) (`self.Number Of Enemies`))
    (else
      (`self.Should Spawn?`))))

(event `Should Spawn?`
  (bind _as_bp_game_mode_base (`self.As BP Game Mode Base`))
  ;[1 1 1] Spawn enemy Logic
  ;;[1 1 1] Loop for Spawning enemies if their count is less than 5
  (`KismetSystemLibrary.Delay` (`self.Spawn Delay`))
  (if (< (`/Game/Blueprints/BP_GameModeBase.Enemies Alive` _as_bp_game_mode_base) (`/Game/Blueprints/BP_GameModeBase.Max Enemies` _as_bp_game_mode_base))
    (`self.Event SpawnEnemy` (`self.Enemy`) (`KismetMathLibrary.MakeTransform` (`SceneComponent.K2_GetComponentLocation` (`KismetArrayLibrary.Array_Random` (`|MakeArray` (`self.SpawnPoint2`) (`self.SpawnPoint1`)))) (struct :`Yaw` -90.0)) (`self.Number Of Enemies`))
    (else
      (`self.Should Spawn?`))))

(fn `UserConstructionScript`)