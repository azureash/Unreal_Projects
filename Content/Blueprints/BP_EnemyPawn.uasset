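; BP_EnemyPawn is an enemy pawn with a simple health system that reports its spawn and death to the game mode.
; On BeginPlay it calls SpawnEnemies on BP_GameModeBase to register itself in the enemy count.
; The HitEnemy event subtracts damage from Health and, at zero or below, destroys the actor and calls KillEnemies on the game mode to lower that count.
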(event `/Game/Blueprints/BP_EnemyDamage_Interface.HitEnemy`
  (params (Damage :type Integer))
  ;[1 1 1] Enemy Health System
  (bind _output_get (set `self.Health` (- (`self.Health`) Damage)))
  (if (<= _output_get 0)
    (`self.K2_DestroyActor`)
    ;[1 1 1] As enemy dies, decrease enemy count by 1
    (bind _asbp_game_mode_base (cast `/Game/Blueprints/BP_GameModeBase` (`GameplayStatics.GetGameMode`)))
    (`/Game/Blueprints/BP_GameModeBase.Kill Enemies` _asbp_game_mode_base)))

(event `self.ReceiveBeginPlay`
  ;[1 1 1] At first enemy spawn, count increases by 1
  (bind _asbp_game_mode_base (cast `/Game/Blueprints/BP_GameModeBase` (`GameplayStatics.GetGameMode`)))
  (`/Game/Blueprints/BP_GameModeBase.Spawn Enemies` _asbp_game_mode_base))

(fn `UserConstructionScript`)